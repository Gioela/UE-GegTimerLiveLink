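; BP_WallClock is an analog wall clock with text readouts, driven by Live Link time data and offset by a configurable time zone.
; On BeginPlay it builds the UTC label from the signed TimeZone value.
; Each Live Link update reads Basic role time properties to roll the three hands and refresh the time text.
; MinutesIncreaser offsets the minutes, and the hour hand advances proportionally with them.
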(event OnLiveLinkUpdated(LiveLinkComponentController)
  (params (DeltaTime :type Float%20%28single-precision%29))
  (bind _houreulerangle (Variables|CoreSettings|GetHourEulerAngle))
  (bind _krotation1min (Variables|CoreSettings|GetKRotation1Min))
  (bind _dataresult (|EvaluateLiveLinkFramewithSpecificRole "(Name=\"Time\")" "/Script/LiveLinkInterface.LiveLinkBasicRole")
    (:then
      (Transformation|SetRelativeRotation (Variables|Default|GetOSeconds) (Math|Rotator|MakeRotator (* (.Value (Class|LiveLinkBlueprintLibrary|GetPropertyValue _dataresult "Seconds")) _krotation1min) 0.0 0.0) false false)
      (Transformation|SetRelativeRotation (Variables|Default|GetOMinutes) (Math|Rotator|MakeRotator (* _krotation1min (+ (.Value (Class|LiveLinkBlueprintLibrary|GetPropertyValue _dataresult "Minutes")) (Variables|PropertySettings|GetMinutesIncreaser))) 0.0 0.0) false false)
      (Transformation|SetRelativeRotation (Variables|Default|GetOHours) (Math|Rotator|MakeRotator (+ (/ (* (* _krotation1min (+ (.Value (Class|LiveLinkBlueprintLibrary|GetPropertyValue _dataresult "Minutes")) (Variables|PropertySettings|GetMinutesIncreaser))) _houreulerangle) (Variables|CoreSettings|GetEulerRoundCorner)) (* (* _houreulerangle -1.0) (+ (Math|Conversions|ToFloat(Integer) (Variables|PropertySettings|GetTimeZone)) (.Value (Class|LiveLinkBlueprintLibrary|GetPropertyValue _dataresult "Hours12"))))) 0.0 0.0) false false)
      (Rendering|Components|TextRender|SetText (Variables|Default|GetUTCTime) (Utilities|Text|ToText(String) (Utilities|String|Append (Utilities|String|ToString(Integer) (Math|Conversions|ToInteger(Byte) (Class|KismetMathLibrary|FTrunc64 (+ (Math|Conversions|ToFloat(Integer) (Variables|PropertySettings|GetTimeZone)) (.Value (Class|LiveLinkBlueprintLibrary|GetPropertyValue _dataresult "Hours12")))))) ":" (Utilities|String|ToString(Integer) (Math|Conversions|ToInteger(Byte) (Class|KismetMathLibrary|FTrunc64 (+ (.Value (Class|LiveLinkBlueprintLibrary|GetPropertyValue _dataresult "Minutes")) (Variables|PropertySettings|GetMinutesIncreaser))))) "." (Utilities|String|ToString(Integer) (Math|Conversions|ToInteger(Byte) (Class|KismetMathLibrary|FTrunc64 (.Value (Class|LiveLinkBlueprintLibrary|GetPropertyValue _dataresult "Seconds")))))))))))

(event EventBeginPlay
  (bind _utclabel (Variables|Default|GetUTCLabel))
  (bind _timezone (Variables|PropertySettings|GetTimeZone))
  (bind _timezonelabel (Variables|PropertySettings|GetTimeZoneLabel))
  (if (== _timezone 0)
    (Rendering|Components|TextRender|SetText (Variables|Default|GetUTCLabel) (Utilities|Text|ToText(String) _timezonelabel))
    (elif (> _timezone 0)
      (Rendering|Components|TextRender|SetText _utclabel (Utilities|Text|ToText(String) (Utilities|String|Append _timezonelabel " +" (Utilities|String|ToString(Integer) _timezone))))
      (else
        (Rendering|Components|TextRender|SetText _utclabel (Utilities|Text|ToText(String) (Utilities|String|Append (Variables|PropertySettings|GetTimeZoneLabel) " " (Utilities|String|ToString(Integer) _timezone))))))))

(fn ConstructionScript)